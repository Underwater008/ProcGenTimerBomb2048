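; Overhead spawner for the TimerBomb game that drops BP_BombMaster bombs until GameOver.
; Spawn retries random XY offsets until inside the play bounds, then attaches a new bomb with a random or fixed level.
; A self-restarting ReleaseTimer detaches it with physics and sound, spawns the next after a delay, and runs a Seconds countdown.
; Tick supports sideways movement, but the logic that sets Move is unwired.
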(event Custom|_ReleaseTimer
  (bind _bp_fruit (Variables|Default|GetBP%20Fruit))
  (bind _box (Variables|/Game/TimerBomb/BP_BombMaster.BP_BombMaster_C|GetBox _bp_fruit))
  ;[1 1 1] Control
  (if (not (Variables|Default|GetGameOver))
    (Utilities|IsValid _bp_fruit
      (:Is%20Valid
        (Physics|SetSimulatePhysics _box true)
        (Variables|/Game/TimerBomb/BP_BombMaster.BP_BombMaster_C|SetSimulate _bp_fruit true)
        (Collision|SetCollisionEnabled _box "QueryAndPhysics")
        (Transformation|DetachFromActor _bp_fruit "KeepWorld" "KeepWorld" "KeepWorld")
        (Utilities|FlowControl|Sequence
          (:then_0
            (Audio|PlaySound2D "/Game/Square/Audio/下落.下落" 1.0 1.0 0.0 0 0)
            (Utilities|FlowControl|Delay (Math|Random|RandomFloatinRange 1.0 1.0))
            (CallFunction|Spawn)
            (Utilities|FlowControl|Delay (Math|Random|RandomFloatinRange 1.0 1.0))
            (CallFunction|ReleaseTimer))
          (:then_1
            ;[1 1 1] Timer
            (Utilities|FlowControl|Delay 1.0 :!label _label)
            (if (not (== (Variables|Default|GetSeconds) 0))
              (Variables|Default|SetSeconds (- (Variables|Default|GetSeconds) 1))
              (goto _label))))))))

(event EventBeginPlay
  (Input|EnableInput (Game|GetPlayerController 0))
  (CallFunction|Spawn)
  (Utilities|FlowControl|Delay 0.5)
  (CallFunction|ReleaseTimer))

(event Collision|EventActorBeginOverlap
  (params (OtherActor :type Actor%20Object%20Reference)))

(event EventTick
  (params (DeltaSeconds :type Float%20%28single-precision%29))
  (bind _returnvalue (Transformation|GetActorRightVector))
  (if (Variables|Default|GetMove)
    (Transformation|AddActorWorldOffset (select (Variables|Default|GetLeft/Right) (* _returnvalue -5.0) (* _returnvalue 5.0)))))

(event Input|KeyboardEvents|A
  (params (Key :type Key%20Structure :default "None"))
  ;[1 1 1] Control
)

(event Input|KeyboardEvents|D
  (params (Key :type Key%20Structure :default "None"))
  ;[1 1 1] Control
)

(event Input|KeyboardEvents|SpaceBar
  (params (Key :type Key%20Structure :default "None"))
  ;[1 1 1] Control
)

(fn ConstructionScript)

(fn Spawn
  (Utilities|FlowControl|Sequence :!label _label
    (:then_0
      (Variables|Default|Setx%20Value (+ (.X (Math|Vector|BreakVector (Transformation|GetActorLocation))) (Math|Random|RandomIntegerinRange -500 500))))
    (:then_1
      (Variables|Default|Sety%20Value (+ (.Y (Math|Vector|BreakVector (Transformation|GetActorLocation))) (Math|Random|RandomIntegerinRange -500 500))))
    (:then_2
      (if (Math|Float|InRange(Float) (Variables|Default|Getx%20Value) 1e+02 1.4e+03)
        (if (Math|Float|InRange(Float) (Variables|Default|Gety%20Value) 1e+02 1.4e+03)
          (Transformation|SetActorLocation (Math|Vector|MakeVector (Variables|Default|Getx%20Value) (Variables|Default|Gety%20Value) 7.5e+02) false false)
          (bind _returnvalue (Game|SpawnActorfromClass "/Game/TimerBomb/BP_BombMaster.BP_BombMaster_C" (Math|Transform|MakeTransform (Transformation|GetActorLocation) "0, 0, 0" "1.000000,1.000000,1.000000") "AlwaysSpawn" 0 (select (Variables|Default|Get随机模式) (.OutItem (Utilities|Array|Random (Utilities|Array|MakeArray "NewEnumerator0" "NewEnumerator1" "NewEnumerator2" "NewEnumerator3" "NewEnumerator4" "NewEnumerator5"))) (Variables|Default|Get固定生成)) (Variables|Default|Get游戏模式) false 1000 9999 (Variables|Default|Gethp) 1 0))
          (bind _output_get (Variables|Default|SetBP%20Fruit _returnvalue))
          (Variables|/Game/TimerBomb/BP_BombMaster.BP_BombMaster_C|SetTrace _output_get false)
          (Transformation|AttachActorToActor _output_get self "None" "KeepWorld" "KeepWorld" "KeepWorld" true)
          (Collision|SetCollisionEnabled (Variables|/Game/TimerBomb/BP_BombMaster.BP_BombMaster_C|GetBox _output_get) "QueryAndPhysics")
          (else
            (goto _label)))
        (else
          (goto _label))))))