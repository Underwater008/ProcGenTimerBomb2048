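; Timed bomb ball that merges with same-level bombs and explodes when its per-level countdown runs out.
; On a hit, a random ID picks the survivor, which animates to the next level's geometrically scaled size, resets its countdown, and shatters at top levels.
; At zero it shakes the camera, pushes bombs and the player tracked by an overlap sphere, and damages the player.
; Game mode selects the mesh, and level selects the material.
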(event OnComponentHit(Sphere)
  (params (HitComponent :type Primitive%20Component%20Object%20Reference) (OtherActor :type Actor%20Object%20Reference) (OtherComp :type Primitive%20Component%20Object%20Reference) (NormalImpulse :type Vector :default "0, 0, 0") (Hit :type Hit%20Result%20Structure%20%28by%20ref%29))
  (bind _asbp_bomb_master (Utilities|Casting|CastToBP_BombMaster OtherActor))
  (if (not (Variables|BP_BombMaster_C|GetIsUping _asbp_bomb_master))
    (if (Utilities|Enum|Equal(Enum) (Variables|BP_BombMaster_C|GetLevel _asbp_bomb_master) (Variables|Default|GetLevel))
      (if (not (> (Variables|/Game/Combine/BP/BPC_LevelType.BPC_LevelType_C|GetID (Variables|BP_BombMaster_C|GetBPC_Level _asbp_bomb_master)) (Variables|/Game/Combine/BP/BPC_LevelType.BPC_LevelType_C|GetID (Variables|Default|GetBPC_Level))))
        (Variables|Default|SetIsUping true)
        (Utilities|FlowControl|DoOnce false
          (:Completed
            (Utilities|FlowControl|Sequence
              (:then_0
                (CallFunction|动画))
              (:then_1
                (Actor|DestroyActor _asbp_bomb_master)
                (if (>= (Variables|Default|GetLevel) 5)
                  (CallFunction|破碎)))
              (:then_2
                (if (not (Variables|Default|GetTrace))
                  (Audio|PlaySound2D "/Game/Square/Audio/土砖掉落.土砖掉落" 0.5 1.0 0.0 0 0)))
              (:then_3
                (Variables|Default|SetIsUping false))
              (:then_4
                (bind _output_get (Variables|Default|SetSeconds (Utilities|Select :Index (Variables|Default|GetLevel) :NewEnumerator0 5 :NewEnumerator1 10 :NewEnumerator2 15 :NewEnumerator3 20 :NewEnumerator4 25 :NewEnumerator5 30 :NewEnumerator6 10)))
                (Variables|Default|SetLastSeconds _output_get)))))))))

(event OnComponentHit(Box)
  (params (HitComponent :type Primitive%20Component%20Object%20Reference) (OtherActor :type Actor%20Object%20Reference) (OtherComp :type Primitive%20Component%20Object%20Reference) (NormalImpulse :type Vector :default "0, 0, 0") (Hit :type Hit%20Result%20Structure%20%28by%20ref%29)))

(event OnComponentBeginOverlap(Sphere1)
  (params (OverlappedComponent :type Primitive%20Component%20Object%20Reference) (OtherActor :type Actor%20Object%20Reference) (OtherComp :type Primitive%20Component%20Object%20Reference) (OtherBodyIndex :type Integer) (bFromSweep :type Boolean) (SweepResult :type Hit%20Result%20Structure%20%28by%20ref%29))
  (bind _balls (Variables|Default|GetBalls))
  (Utilities|FlowControl|Sequence
    (:then_0
      (bind _asbp_top_down_character (Utilities|Casting|CastToBP_TopDownCharacter OtherActor))
      (Variables|Default|SetAs%20BP%20Top%20Down%20Character _asbp_top_down_character))
    (:then_1
      (bind _asbp_bomb_master (Utilities|Casting|CastToBP_BombMaster OtherActor))
      (if (== (Utilities|Array|FindItem _balls _asbp_bomb_master) -1)
        (Utilities|Array|Add _balls _asbp_bomb_master)))))

(event OnComponentEndOverlap(Sphere1)
  (params (OverlappedComponent :type Primitive%20Component%20Object%20Reference) (OtherActor :type Actor%20Object%20Reference) (OtherComp :type Primitive%20Component%20Object%20Reference) (OtherBodyIndex :type Integer))
  (bind _balls (Variables|Default|GetBalls))
  (Utilities|FlowControl|Sequence
    (:then_0
      (Utilities|Casting|CastToBP_TopDownCharacter OtherActor)
      (Variables|Default|SetAs%20BP%20Top%20Down%20Character 0))
    (:then_1
      (bind _asbp_bomb_master (Utilities|Casting|CastToBP_BombMaster OtherActor))
      (Utilities|IsValid (Utilities|Array|Get(acopy) _balls (Utilities|Array|FindItem (Variables|Default|GetBalls) _asbp_bomb_master))
        (:Is%20Valid
          (Utilities|Array|RemoveItem _balls (Utilities|Array|Get(acopy) _balls (Utilities|Array|FindItem (Variables|Default|GetBalls) _asbp_bomb_master))))))))

(event Custom|动画
  (bind _基准倍率 (Variables|Default|Get基准倍率))
  (bind _基准倍率_2 (Variables|Default|Get基准倍率))
  (bind _基准缩放 (Variables|Default|Get基准缩放))
  (bind _基准范围 (Variables|Default|Get基准范围))
  (bind _基准倍率_3 (Variables|Default|Get基准倍率))
  (bind _基准倍率_4 (Variables|Default|Get基准倍率))
  (bind _基准缩放_2 (Variables|Default|Get基准缩放))
  (bind _基准范围_2 (Variables|Default|Get基准范围))
  (bind (_l1 _l2 _l3 _l4 _l5 _l6) (CallFunction|倍率 _基准范围 _基准倍率_3))
  (bind (_l1_2 _l2_2 _l3_2 _l4_2 _l5_2 _l6_2) (CallFunction|倍率 _基准缩放_2 _基准倍率_4))
  (bind (_l1_3 _l2_3 _l3_3 _l4_3 _l5_3 _l6_3) (CallFunction|倍率 _基准缩放 _基准倍率_2))
  (bind (_l1_4 _l2_4 _l3_4 _l4_4 _l5_4 _l6_4) (CallFunction|倍率 _基准范围_2 _基准倍率))
  ;[1 1 1] 动画
  (Variables|Default|Set当前范围 (Utilities|Select :Index (Variables|Default|GetLevel) :NewEnumerator0 _l1_4 :NewEnumerator1 _l2_4 :NewEnumerator2 _l3_4 :NewEnumerator3 _l4_4 :NewEnumerator4 _l5_4 :NewEnumerator5 _l6_4 :NewEnumerator6 "0, 0, 0"))
  (Variables|Default|Set当前缩放 (Utilities|Select :Index (Variables|Default|GetLevel) :NewEnumerator0 _l1_3 :NewEnumerator1 _l2_3 :NewEnumerator2 _l3_3 :NewEnumerator3 _l4_3 :NewEnumerator4 _l5_3 :NewEnumerator5 _l6_3 :NewEnumerator6 "0, 0, 0"))
  (Variables|Default|Set新范围 (Utilities|Select :Index (Utilities|Enum|ByteToEnumEnum_Level (Math|Conversions|ToByte(Integer) (+ (Math|Conversions|ToInteger(Byte) (Variables|Default|GetLevel)) 1))) :NewEnumerator0 _l1 :NewEnumerator1 _l2 :NewEnumerator2 _l3 :NewEnumerator3 _l4 :NewEnumerator4 _l5 :NewEnumerator5 _l6 :NewEnumerator6 "0, 0, 0"))
  (Variables|Default|Set新缩放 (Utilities|Select :Index (Utilities|Enum|ByteToEnumEnum_Level (Math|Conversions|ToByte(Integer) (+ (Math|Conversions|ToInteger(Byte) (Variables|Default|GetLevel)) 1))) :NewEnumerator0 _l1_2 :NewEnumerator1 _l2_2 :NewEnumerator2 _l3_2 :NewEnumerator3 _l4_2 :NewEnumerator4 _l5_2 :NewEnumerator5 _l6_2 :NewEnumerator6 "0, 0, 0"))
  (Components|Timeline|SetPlayRate (Variables|Default|GetScale) (Variables|Default|Get动画速度))
  (bind _scale (Timeline|Scale PlayFromStart)
    (:Update
      (Components|Sphere|SetSphereRadius (Variables|Default|GetSphere) (.X (Math|Vector|BreakVector (Math|Vector|Lerp(Vector) (Variables|Default|Get当前范围) (Variables|Default|Get新范围) _scale))) true)
      (Transformation|SetRelativeScale3D (Variables|Default|GetSM_RCube) (Math|Vector|Lerp(Vector) (Variables|Default|Get当前缩放) (Variables|Default|Get新缩放) _scale)))
    (:Finished
      (Variables|Default|SetLevel (Utilities|Enum|ByteToEnumEnum_Level (Math|Conversions|ToByte(Integer) (+ (Math|Conversions|ToInteger(Byte) (Variables|Default|GetLevel)) 1))))
      (CallFunction|Refresh))))

(event Custom|自定义事件_0
  (bind _as_bp_top_down_character (Variables|Default|GetAs%20BP%20Top%20Down%20Character))
  (bind _result (Math|Integer|DecrementInt (Variables|Default|GetSeconds))
    (:%20%20
      (if (< _result 1)
        (Utilities|Time|ClearandInvalidateTimerbyHandle (Variables|Default|GetTimerEvent))
        (Variables|Default|SetSimulate true)
        (Effects|SpawnEmitteratLocation "/Game/StarterContent/Particles/P_Explosion.P_Explosion" (Transformation|GetWorldLocation (Variables|Default|GetSM_RCube)))
        (Game|Feedback|ClientStartCameraShake (Game|GetPlayerController 0) "/Game/AAA/NewBlueprint.NewBlueprint_C" 4.0 "CameraLocal" "0, 0, 0")
        (Utilities|FlowControl|Sequence
          (:then_0
            (if (Utilities|Array|IsValidIndex (Variables|Default|GetBalls))
              (for _array_element (Variables|Default|GetBalls)
                (Physics|AddImpulse (Variables|BP_BombMaster_C|GetSphere _array_element) (* (Math|Rotator|GetRotationXVector (Math|Rotator|FindLookatRotation (Transformation|GetActorLocation) (Transformation|GetActorLocation _array_element))) 1000) "None" true))))
          (:then_1
            (Utilities|IsValid _as_bp_top_down_character
              (:Is%20Valid
                (Default|扣血 _as_bp_top_down_character (Variables|Default|GetDamageValue))
                (Physics|AddImpulse (Variables|/Script/Engine.Character|GetCharacterMovement _as_bp_top_down_character) (* (Math|Rotator|GetRotationXVector (Math|Rotator|FindLookatRotation (Transformation|GetActorLocation) (Transformation|GetActorLocation _as_bp_top_down_character))) 1000) true))
              (:Is%20Not%20Valid
                _))
            (Utilities|FlowControl|Delay 0.2)
            (Actor|DestroyActor)))))))

(event Custom|Refresh
  (Utilities|FlowControl|DoOnce false) ; enters at Reset
)

(event EventBeginPlay
  (Utilities|FlowControl|Sequence
    (:then_0
      (Physics|SetSimulatePhysics (Variables|Default|GetSphere) (Variables|Default|GetSimulate))
      (CallFunction|等级)
      (if (Variables|Default|GetSimulate)
        (Variables|Default|SetTrace true)
        (Utilities|FlowControl|Delay 1.0)
        (Actor|DestroyActor)
        (else
          (Variables|Default|SetTrace false))))
    (:then_1
      (Utilities|FlowControl|Delay 1.0 :!label _label)
      (Rendering|ToggleVisibility (Variables|Default|GetPointLight) false)
      (Utilities|FlowControl|Delay 1.0)
      (Rendering|ToggleVisibility (Variables|Default|GetPointLight) false)
      (goto _label))
    (:then_2
      (bind _asui_bomb_timer (Utilities|Casting|CastToUI_BombTimer (UserInterface|GetUserWidgetObject (Variables|Replication|GetTimer))))
      (Variables|/Game/TimerBomb/UI_BombTimer.UI_BombTimer_C|SetBP_Master _asui_bomb_timer self))
    (:then_3
      (bind _returnvalue (Utilities|Time|SetTimerbyEvent (delegate Custom|自定义事件_0) 1.0 true))
      (Variables|Default|SetTimerEvent _returnvalue))
    (:then_4
      (bind _output_get (Variables|Default|SetSeconds (Utilities|Select :Index (Variables|Default|GetLevel) :NewEnumerator0 5 :NewEnumerator1 10 :NewEnumerator2 15 :NewEnumerator3 20 :NewEnumerator4 25 :NewEnumerator5 30 :NewEnumerator6 10)))
      (Variables|Default|SetLastSeconds _output_get))))

(event Collision|EventActorBeginOverlap
  (params (OtherActor :type Actor%20Object%20Reference)))

(event EventTick
  (params (DeltaSeconds :type Float%20%28single-precision%29))
  (bind _level (Variables|Default|GetLevel))
  (Utilities|FlowControl|Sequence
    (:then_0
      (if (< (Variables|Default|GetLevel) 6)
        _))
    (:then_1
      (Utilities|IsValid self
        (:Is%20Valid
          (Rendering|Material|SetMaterial (Variables|Default|GetSM_RCube) 0 (Utilities|Select :Index (Variables|Default|Get游戏模式) :NewEnumerator0 (Utilities|Select :Index _level :NewEnumerator0 "/Game/TimerBomb/M_TimerBomb_1.M_TimerBomb_1" :NewEnumerator1 "/Game/TimerBomb/M_TimerBomb_2.M_TimerBomb_2" :NewEnumerator2 "/Game/TimerBomb/M_TimerBomb_3.M_TimerBomb_3" :NewEnumerator3 "/Game/TimerBomb/M_TimerBomb_4.M_TimerBomb_4" :NewEnumerator4 "/Game/TimerBomb/M_TimerBomb_5.M_TimerBomb_5" :NewEnumerator5 "/Game/TimerBomb/M_TimerBomb_6.M_TimerBomb_6" :NewEnumerator6 "/Game/TimerBomb/M_TimerBomb_7.M_TimerBomb_7") :NewEnumerator1 (Utilities|Select :Index _level :NewEnumerator0 "/Game/TimerBomb/M_TimerBomb_1.M_TimerBomb_1" :NewEnumerator1 "/Game/TimerBomb/M_TimerBomb_2.M_TimerBomb_2" :NewEnumerator2 "/Game/TimerBomb/M_TimerBomb_3.M_TimerBomb_3" :NewEnumerator3 "/Game/TimerBomb/M_TimerBomb_4.M_TimerBomb_4" :NewEnumerator4 "/Game/TimerBomb/M_TimerBomb_5.M_TimerBomb_5" :NewEnumerator5 "/Game/TimerBomb/M_TimerBomb_6.M_TimerBomb_6" :NewEnumerator6 "/Game/TimerBomb/M_TimerBomb_7.M_TimerBomb_7") :NewEnumerator7 (Utilities|Select :Index _level :NewEnumerator0 "/Game/TimerBomb/M_TimerBomb_1.M_TimerBomb_1" :NewEnumerator1 "/Game/TimerBomb/M_TimerBomb_2.M_TimerBomb_2" :NewEnumerator2 "/Game/TimerBomb/M_TimerBomb_3.M_TimerBomb_3" :NewEnumerator3 "/Game/TimerBomb/M_TimerBomb_4.M_TimerBomb_4" :NewEnumerator4 "/Game/TimerBomb/M_TimerBomb_5.M_TimerBomb_5" :NewEnumerator5 "/Game/TimerBomb/M_TimerBomb_6.M_TimerBomb_6" :NewEnumerator6 "/Game/TimerBomb/M_TimerBomb_7.M_TimerBomb_7"))))))
    (:then_2
      (if (Variables|Default|GetSimulate)
        (Utilities|FlowControl|DoOnce false
          (:Completed
            (Utilities|FlowControl|Delay 2.0)
            (Variables|Default|SetTrace true)))))))

(fn ConstructionScript
  (bind _游戏模式 (Variables|Default|Get游戏模式))
  (Components|StaticMesh|SetStaticMesh (Variables|Default|GetSM_RCube) (Utilities|Select :Index _游戏模式 :NewEnumerator0 "/Game/TimerBomb/bomb1.bomb1" :NewEnumerator1 "/Game/Combine/Mesh/表情方块.表情方块" :NewEnumerator7 "/Game/TimerBomb/bomb1.bomb1"))
  (CallFunction|等级)
  (if (Utilities|Enum|Equal(Enum) _游戏模式 "NewEnumerator7")
    (Variables|Default|Set基准范围 "18.000000,18.000000,18.000000")))

(fn 倍率
  (params (基准 :type Vector) (基准倍率 :type Float%20%28double-precision%29))
  (bind _returnvalue (* 基准 基准倍率))
  (bind _returnvalue_2 (+ 基准 _returnvalue))
  (bind _returnvalue_3 (* _returnvalue_2 基准倍率))
  (bind _returnvalue_4 (+ _returnvalue_2 _returnvalue_3))
  (bind _returnvalue_5 (* _returnvalue_4 基准倍率))
  (bind _returnvalue_6 (+ _returnvalue_4 _returnvalue_5))
  (bind _returnvalue_7 (* _returnvalue_6 基准倍率))
  (bind _returnvalue_8 (+ _returnvalue_6 _returnvalue_7))
  (bind _returnvalue_9 (* _returnvalue_8 基准倍率))
  (bind _returnvalue_10 (+ _returnvalue_8 _returnvalue_9))
  (return 基准 _returnvalue_2 _returnvalue_4 _returnvalue_6 _returnvalue_8 _returnvalue_10 (+ _returnvalue_10 (* _returnvalue_10 基准倍率))))

(fn 等级
  (bind _基准倍率 (Variables|Default|Get基准倍率))
  (bind _基准范围 (Variables|Default|Get基准范围))
  (bind _bpc_level (Variables|Default|GetBPC_Level))
  (bind _基准缩放 (Variables|Default|Get基准缩放))
  (bind _基准倍率_2 (Variables|Default|Get基准倍率))
  (bind (_l1 _l2 _l3 _l4 _l5 _l6) (CallFunction|倍率 _基准缩放 _基准倍率))
  (bind (_l1_2 _l2_2 _l3_2 _l4_2 _l5_2 _l6_2) (CallFunction|倍率 _基准范围 _基准倍率_2))
  (Variables|/Game/Combine/BP/BPC_LevelType.BPC_LevelType_C|SetLevel _bpc_level (Variables|Default|GetLevel))
  (Variables|/Game/Combine/BP/BPC_LevelType.BPC_LevelType_C|SetID _bpc_level (Math|Random|RandomIntegerinRange (Variables|Default|GetID范围最小值) (Variables|Default|GetID范围最大值)))
  (Components|Sphere|SetSphereRadius (Variables|Default|GetSphere) (.X (Math|Vector|BreakVector (Utilities|Select :Index (Variables|Default|GetLevel) :NewEnumerator0 _l1_2 :NewEnumerator1 _l2_2 :NewEnumerator2 _l3_2 :NewEnumerator3 _l4_2 :NewEnumerator4 _l5_2 :NewEnumerator5 _l6_2 :NewEnumerator6 "0, 0, 0"))) true)
  (Transformation|SetRelativeScale3D (Variables|Default|GetSM_RCube) (Utilities|Select :Index (Variables|Default|GetLevel) :NewEnumerator0 _l1 :NewEnumerator1 _l2 :NewEnumerator2 _l3 :NewEnumerator3 _l4 :NewEnumerator4 _l5 :NewEnumerator5 _l6 :NewEnumerator6 "0, 0, 0"))
  (Rendering|Material|SetMaterial (Variables|Default|GetSM_RCube) 0 (Utilities|Select :Index (Variables|Default|Get游戏模式) :NewEnumerator0 (Utilities|Select :Index (Variables|Default|GetLevel) :NewEnumerator0 "/Game/TimerBomb/M_TimerBomb_1.M_TimerBomb_1" :NewEnumerator1 "/Game/TimerBomb/M_TimerBomb_2.M_TimerBomb_2" :NewEnumerator2 "/Game/TimerBomb/M_TimerBomb_3.M_TimerBomb_3" :NewEnumerator3 "/Game/TimerBomb/M_TimerBomb_4.M_TimerBomb_4" :NewEnumerator4 "/Game/TimerBomb/M_TimerBomb_5.M_TimerBomb_5" :NewEnumerator5 "/Game/TimerBomb/M_TimerBomb_6.M_TimerBomb_6" :NewEnumerator6 "/Game/TimerBomb/M_TimerBomb_7.M_TimerBomb_7") :NewEnumerator1 (Utilities|Select :Index (Variables|Default|GetLevel) :NewEnumerator0 "/Game/TimerBomb/M_TimerBomb_1.M_TimerBomb_1" :NewEnumerator1 "/Game/TimerBomb/M_TimerBomb_2.M_TimerBomb_2" :NewEnumerator2 "/Game/TimerBomb/M_TimerBomb_3.M_TimerBomb_3" :NewEnumerator3 "/Game/TimerBomb/M_TimerBomb_4.M_TimerBomb_4" :NewEnumerator4 "/Game/TimerBomb/M_TimerBomb_5.M_TimerBomb_5" :NewEnumerator5 "/Game/TimerBomb/M_TimerBomb_6.M_TimerBomb_6" :NewEnumerator6 "/Game/TimerBomb/M_TimerBomb_7.M_TimerBomb_7") :NewEnumerator7 (Utilities|Select :Index (Variables|Default|GetLevel) :NewEnumerator0 "/Game/TimerBomb/M_TimerBomb_1.M_TimerBomb_1" :NewEnumerator1 "/Game/TimerBomb/M_TimerBomb_2.M_TimerBomb_2" :NewEnumerator2 "/Game/TimerBomb/M_TimerBomb_3.M_TimerBomb_3" :NewEnumerator3 "/Game/TimerBomb/M_TimerBomb_4.M_TimerBomb_4" :NewEnumerator4 "/Game/TimerBomb/M_TimerBomb_5.M_TimerBomb_5" :NewEnumerator5 "/Game/TimerBomb/M_TimerBomb_6.M_TimerBomb_6" :NewEnumerator6 "/Game/TimerBomb/M_TimerBomb_7.M_TimerBomb_7"))))

(fn 破碎
  (Utilities|FlowControl|DoOnce false
    (:Completed
      (Audio|PlaySound2D "/Game/Square/Audio/消除_.消除_" 0.5 1.0 0.0 0 0)
      (Effects|SpawnEmitteratLocation "/Game/Combine/FX/PS_BlastSmoke.PS_BlastSmoke" (Transformation|GetActorLocation) "0, 0, 0" "0.700000,0.700000,0.700000")
      (Actor|SetLifeSpan 1.0))))

(fn CountDown)