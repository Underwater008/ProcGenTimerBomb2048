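; BP_FruitPlayerPawn is the player pawn in the Combine fruit folder, providing a cine camera and spring arm for the view.
; Its construction script applies exposed variables for arm length and focal length.
; A screen-ratio selector switches the filmback between 16:9 landscape, 9:16 portrait and a custom sensor size.
; BeginPlay and Tick are empty, and a cursor hit-test under player controller 0 is left unconnected.
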(event EventBeginPlay)

(event EventTick
  (params (DeltaSeconds :type Float%20%28single-precision%29)))

(event Input|MouseEvents|LeftMouseButton
  (params (Key :type Key%20Structure :default "None")))

(fn ConstructionScript
  (Variables|/Script/Engine.SpringArmComponent|SetTargetArmLength (Variables|Default|GetSpringArm) (Variables|Default|Get目标臂长度))
  (Variables|/Script/CinematicCamera.CineCameraComponent|SetCurrentFocalLength (Variables|Default|GetCineCamera) (Variables|Default|Get相机焦距))
  (Variables|/Script/CinematicCamera.CineCameraComponent|SetFilmback (Variables|Default|GetCineCamera) (Utilities|Select :Index (Variables|Default|Get相机屏幕比) :Option%200 (Utilities|Struct|MakeCameraFilmbackSettings 19.200001 10.8) :Option%201 (Utilities|Struct|MakeCameraFilmbackSettings 10.8 19.200001) :Option%202 (Utilities|Struct|MakeCameraFilmbackSettings (Variables|Default|Get自定义宽度) (Variables|Default|Get自定义高度)))))