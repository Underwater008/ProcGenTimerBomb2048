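; BP_FruitMaster is a physics merge piece with gem, emoji or funny-ball skins selected by game mode.
; When same-level pieces collide, a random BPCLevel ID picks the survivor, which destroys the other and grows via a timeline before levelling up.
; 倍率 compounds base extent and scale per level, while Tick keeps the material matched to level.
; Merges at top level also trigger 破碎: sound, smoke burst and short lifespan.
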(event OnComponentHit(Box)
  (params (HitComponent :type Primitive%20Component%20Object%20Reference) (OtherActor :type Actor%20Object%20Reference) (OtherComp :type Primitive%20Component%20Object%20Reference) (NormalImpulse :type Vector :default "0, 0, 0") (Hit :type Hit%20Result%20Structure%20%28by%20ref%29))
  (bind _asbp_fruit_master (Utilities|Casting|CastToBP_FruitMaster OtherActor))
  (if (Utilities|Enum|Equal(Enum) (Variables|BP_FruitMaster_C|GetLevel _asbp_fruit_master) (Variables|Default|GetLevel))
    (if (not (> (Variables|/Game/Combine/BP/BPC_LevelType.BPC_LevelType_C|GetID (Variables|BP_FruitMaster_C|GetBPC_Level _asbp_fruit_master)) (Variables|/Game/Combine/BP/BPC_LevelType.BPC_LevelType_C|GetID (Variables|Default|GetBPC_Level))))
      (Utilities|FlowControl|DoOnce false
        (:Completed
          (Utilities|FlowControl|Sequence
            (:then_0
              (CallFunction|动画))
            (:then_1
              (Actor|DestroyActor _asbp_fruit_master)
              (if (>= (Variables|Default|GetLevel) 5)
                (CallFunction|破碎)))
            (:then_2
              (if (not (Variables|Default|GetTrace))
                (Audio|PlaySound2D "/Game/Square/Audio/土砖掉落.土砖掉落" 0.5 1.0 0.0 0 0)))))))))

(event Custom|动画
  (bind _基准倍率 (Variables|Default|Get基准倍率))
  (bind _基准倍率_2 (Variables|Default|Get基准倍率))
  (bind _基准缩放 (Variables|Default|Get基准缩放))
  (bind _基准范围 (Variables|Default|Get基准范围))
  (bind _基准倍率_3 (Variables|Default|Get基准倍率))
  (bind _基准倍率_4 (Variables|Default|Get基准倍率))
  (bind _基准缩放_2 (Variables|Default|Get基准缩放))
  (bind _基准范围_2 (Variables|Default|Get基准范围))
  (bind (_l1 _l2 _l3 _l4 _l5 _l6) (CallFunction|倍率 _基准范围 _基准倍率_3))
  (bind (_l1_2 _l2_2 _l3_2 _l4_2 _l5_2 _l6_2) (CallFunction|倍率 _基准缩放_2 _基准倍率_4))
  (bind (_l1_3 _l2_3 _l3_3 _l4_3 _l5_3 _l6_3) (CallFunction|倍率 _基准缩放 _基准倍率_2))
  (bind (_l1_4 _l2_4 _l3_4 _l4_4 _l5_4 _l6_4) (CallFunction|倍率 _基准范围_2 _基准倍率))
  ;[1 1 1] 动画
  (Variables|Default|Set当前范围 (Utilities|Select :Index (Variables|Default|GetLevel) :NewEnumerator0 _l1_4 :NewEnumerator1 _l2_4 :NewEnumerator2 _l3_4 :NewEnumerator3 _l4_4 :NewEnumerator4 _l5_4 :NewEnumerator5 _l6_4 :NewEnumerator6 "0, 0, 0"))
  (Variables|Default|Set当前缩放 (Utilities|Select :Index (Variables|Default|GetLevel) :NewEnumerator0 _l1_3 :NewEnumerator1 _l2_3 :NewEnumerator2 _l3_3 :NewEnumerator3 _l4_3 :NewEnumerator4 _l5_3 :NewEnumerator5 _l6_3 :NewEnumerator6 "0, 0, 0"))
  (Variables|Default|Set新范围 (Utilities|Select :Index (Utilities|Enum|ByteToEnumEnum_Level (Math|Conversions|ToByte(Integer) (+ (Math|Conversions|ToInteger(Byte) (Variables|Default|GetLevel)) 1))) :NewEnumerator0 _l1 :NewEnumerator1 _l2 :NewEnumerator2 _l3 :NewEnumerator3 _l4 :NewEnumerator4 _l5 :NewEnumerator5 _l6 :NewEnumerator6 "0, 0, 0"))
  (Variables|Default|Set新缩放 (Utilities|Select :Index (Utilities|Enum|ByteToEnumEnum_Level (Math|Conversions|ToByte(Integer) (+ (Math|Conversions|ToInteger(Byte) (Variables|Default|GetLevel)) 1))) :NewEnumerator0 _l1_2 :NewEnumerator1 _l2_2 :NewEnumerator2 _l3_2 :NewEnumerator3 _l4_2 :NewEnumerator4 _l5_2 :NewEnumerator5 _l6_2 :NewEnumerator6 "0, 0, 0"))
  (Components|Timeline|SetPlayRate (Variables|Default|GetScale) (Variables|Default|Get动画速度))
  (bind _scale (Timeline|Scale PlayFromStart)
    (:Update
      (Components|Box|SetBoxExtent (Variables|Default|GetBox) (Math|Vector|Lerp(Vector) (Variables|Default|Get当前范围) (Variables|Default|Get新范围) _scale) false)
      (Transformation|SetRelativeScale3D (Variables|Default|GetSM_RCube) (Math|Vector|Lerp(Vector) (Variables|Default|Get当前缩放) (Variables|Default|Get新缩放) _scale)))
    (:Finished
      (Variables|Default|SetLevel (Utilities|Enum|ByteToEnumEnum_Level (Math|Conversions|ToByte(Integer) (+ (Math|Conversions|ToInteger(Byte) (Variables|Default|GetLevel)) 1))))
      (CallFunction|Refresh))))

(event Custom|Refresh
  (Utilities|FlowControl|DoOnce false) ; enters at Reset
)

(event EventBeginPlay
  (Physics|SetSimulatePhysics (Variables|Default|GetBox) (Variables|Default|GetSimulate))
  (CallFunction|等级)
  (if (Variables|Default|GetSimulate)
    (Variables|Default|SetTrace true)
    (else
      (Variables|Default|SetTrace false))))

(event Collision|EventActorBeginOverlap
  (params (OtherActor :type Actor%20Object%20Reference)))

(event EventTick
  (params (DeltaSeconds :type Float%20%28single-precision%29))
  (bind _level (Variables|Default|GetLevel))
  (Utilities|FlowControl|Sequence
    (:then_0
      (if (< (Variables|Default|GetLevel) 6)
        _))
    (:then_1
      (Utilities|IsValid self
        (:Is%20Valid
          (Rendering|Material|SetMaterial (Variables|Default|GetSM_RCube) 0 (Utilities|Select :Index (Variables|Default|Get游戏模式) :NewEnumerator0 (Utilities|Select :Index _level :NewEnumerator0 "/Game/模型材质/220322方块小游戏/M_Crystal_Inst2_3.M_Crystal_Inst2_3" :NewEnumerator1 "/Game/模型材质/220322方块小游戏/M_Crystal_Inst6_2.M_Crystal_Inst6_2" :NewEnumerator2 "/Game/模型材质/220322方块小游戏/M_Crystal_Inst4_2.M_Crystal_Inst4_2" :NewEnumerator3 "/Game/模型材质/220322方块小游戏/M_Crystal_Inst5_3.M_Crystal_Inst5_3" :NewEnumerator4 "/Game/模型材质/220322方块小游戏/M_Crystal_Inst7_2.M_Crystal_Inst7_2" :NewEnumerator5 "/Game/模型材质/220322方块小游戏/M_Crystal_Inst3_2.M_Crystal_Inst3_2" :NewEnumerator6 0) :NewEnumerator1 (Utilities|Select :Index _level :NewEnumerator0 "/Game/Combine/Mat/01_Inst.01_Inst" :NewEnumerator1 "/Game/Combine/Mat/02_Inst.02_Inst" :NewEnumerator2 "/Game/Combine/Mat/03_Inst.03_Inst" :NewEnumerator3 "/Game/Combine/Mat/04_Inst.04_Inst" :NewEnumerator4 "/Game/Combine/Mat/05_Inst.05_Inst" :NewEnumerator5 "/Game/Combine/Mat/06_Inst.06_Inst" :NewEnumerator6 0) :NewEnumerator7 (Utilities|Select :Index _level :NewEnumerator0 "/Game/Combine/Mat/M_BQ_Inst2.M_BQ_Inst2" :NewEnumerator1 "/Game/Combine/Mat/M_BQ_Inst3.M_BQ_Inst3" :NewEnumerator2 "/Game/Combine/Mat/M_BQ_Inst4.M_BQ_Inst4" :NewEnumerator3 "/Game/Combine/Mat/M_BQ_Inst5.M_BQ_Inst5" :NewEnumerator4 "/Game/Combine/Mat/M_BQ_Inst7.M_BQ_Inst7" :NewEnumerator5 "/Game/Combine/Mat/M_BQ_Inst6.M_BQ_Inst6" :NewEnumerator6 0))))))
    (:then_2
      (if (Variables|Default|GetSimulate)
        (Utilities|FlowControl|DoOnce false
          (:Completed
            (Utilities|FlowControl|Delay 2.0)
            (Variables|Default|SetTrace true)))))))

(fn ConstructionScript
  (bind _游戏模式 (Variables|Default|Get游戏模式))
  (Components|StaticMesh|SetStaticMesh (Variables|Default|GetSM_RCube) (Utilities|Select :Index _游戏模式 :NewEnumerator0 "/Game/Combine/Mesh/SM_RCube.SM_RCube" :NewEnumerator1 "/Game/Combine/Mesh/表情方块.表情方块" :NewEnumerator7 "/Game/Combine/Mesh/表情球.表情球"))
  (CallFunction|等级)
  (if (Utilities|Enum|Equal(Enum) _游戏模式 "NewEnumerator7")
    (Variables|Default|Set基准范围 "18.000000,18.000000,18.000000")))

(fn 倍率
  (params (基准 :type Vector) (基准倍率 :type Float%20%28double-precision%29))
  (bind _returnvalue (* 基准 基准倍率))
  (bind _returnvalue_2 (+ 基准 _returnvalue))
  (bind _returnvalue_3 (* _returnvalue_2 基准倍率))
  (bind _returnvalue_4 (+ _returnvalue_2 _returnvalue_3))
  (bind _returnvalue_5 (* _returnvalue_4 基准倍率))
  (bind _returnvalue_6 (+ _returnvalue_4 _returnvalue_5))
  (bind _returnvalue_7 (* _returnvalue_6 基准倍率))
  (bind _returnvalue_8 (+ _returnvalue_6 _returnvalue_7))
  (bind _returnvalue_9 (* _returnvalue_8 基准倍率))
  (bind _returnvalue_10 (+ _returnvalue_8 _returnvalue_9))
  (return 基准 _returnvalue_2 _returnvalue_4 _returnvalue_6 _returnvalue_8 _returnvalue_10 (+ _returnvalue_10 (* _returnvalue_10 基准倍率))))

(fn 等级
  (bind _基准倍率 (Variables|Default|Get基准倍率))
  (bind _基准范围 (Variables|Default|Get基准范围))
  (bind _bpc_level (Variables|Default|GetBPC_Level))
  (bind _基准缩放 (Variables|Default|Get基准缩放))
  (bind _基准倍率_2 (Variables|Default|Get基准倍率))
  (bind (_l1 _l2 _l3 _l4 _l5 _l6) (CallFunction|倍率 _基准缩放 _基准倍率))
  (bind (_l1_2 _l2_2 _l3_2 _l4_2 _l5_2 _l6_2) (CallFunction|倍率 _基准范围 _基准倍率_2))
  (Variables|/Game/Combine/BP/BPC_LevelType.BPC_LevelType_C|SetLevel _bpc_level (Variables|Default|GetLevel))
  (Variables|/Game/Combine/BP/BPC_LevelType.BPC_LevelType_C|SetID _bpc_level (Math|Random|RandomIntegerinRange (Variables|Default|GetID范围最小值) (Variables|Default|GetID范围最大值)))
  (Components|Box|SetBoxExtent (Variables|Default|GetBox) (Utilities|Select :Index (Variables|Default|GetLevel) :NewEnumerator0 _l1_2 :NewEnumerator1 _l2_2 :NewEnumerator2 _l3_2 :NewEnumerator3 _l4_2 :NewEnumerator4 _l5_2 :NewEnumerator5 _l6_2 :NewEnumerator6 "0, 0, 0") false)
  (Transformation|SetRelativeScale3D (Variables|Default|GetSM_RCube) (Utilities|Select :Index (Variables|Default|GetLevel) :NewEnumerator0 _l1 :NewEnumerator1 _l2 :NewEnumerator2 _l3 :NewEnumerator3 _l4 :NewEnumerator4 _l5 :NewEnumerator5 _l6 :NewEnumerator6 "0, 0, 0"))
  (Rendering|Material|SetMaterial (Variables|Default|GetSM_RCube) 0 (Utilities|Select :Index (Variables|Default|Get游戏模式) :NewEnumerator0 (Utilities|Select :Index (Variables|Default|GetLevel) :NewEnumerator0 "/Game/模型材质/220322方块小游戏/M_Crystal_Inst2_3.M_Crystal_Inst2_3" :NewEnumerator1 "/Game/模型材质/220322方块小游戏/M_Crystal_Inst6_2.M_Crystal_Inst6_2" :NewEnumerator2 "/Game/模型材质/220322方块小游戏/M_Crystal_Inst4_2.M_Crystal_Inst4_2" :NewEnumerator3 "/Game/模型材质/220322方块小游戏/M_Crystal_Inst5_3.M_Crystal_Inst5_3" :NewEnumerator4 "/Game/模型材质/220322方块小游戏/M_Crystal_Inst7_2.M_Crystal_Inst7_2" :NewEnumerator5 "/Game/模型材质/220322方块小游戏/M_Crystal_Inst3_2.M_Crystal_Inst3_2" :NewEnumerator6 0) :NewEnumerator1 (Utilities|Select :Index (Variables|Default|GetLevel) :NewEnumerator0 "/Game/Combine/Mat/01_Inst.01_Inst" :NewEnumerator1 "/Game/Combine/Mat/02_Inst.02_Inst" :NewEnumerator2 "/Game/Combine/Mat/03_Inst.03_Inst" :NewEnumerator3 "/Game/Combine/Mat/04_Inst.04_Inst" :NewEnumerator4 "/Game/Combine/Mat/05_Inst.05_Inst" :NewEnumerator5 "/Game/Combine/Mat/06_Inst.06_Inst" :NewEnumerator6 0) :NewEnumerator7 (Utilities|Select :Index (Variables|Default|GetLevel) :NewEnumerator0 "/Game/Combine/Mat/M_BQ_Inst2.M_BQ_Inst2" :NewEnumerator1 "/Game/Combine/Mat/M_BQ_Inst3.M_BQ_Inst3" :NewEnumerator2 "/Game/Combine/Mat/M_BQ_Inst4.M_BQ_Inst4" :NewEnumerator3 "/Game/Combine/Mat/M_BQ_Inst5.M_BQ_Inst5" :NewEnumerator4 "/Game/Combine/Mat/M_BQ_Inst7.M_BQ_Inst7" :NewEnumerator5 "/Game/Combine/Mat/M_BQ_Inst6.M_BQ_Inst6" :NewEnumerator6 0))))

(fn 破碎
  (Utilities|FlowControl|DoOnce false
    (:Completed
      (Audio|PlaySound2D "/Game/Square/Audio/消除_.消除_" 0.5 1.0 0.0 0 0)
      (Effects|SpawnEmitteratLocation "/Game/Combine/FX/PS_BlastSmoke.PS_BlastSmoke" (Transformation|GetActorLocation) "0, 0, 0" "0.700000,0.700000,0.700000")
      (Actor|SetLifeSpan 1.0))))