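; Deadline trigger volume for the Combine fruit game that decides both defeat and victory, with a configurable box extent.
; After a two-second grace period, Tick checks overlapping BP_FruitMaster actors and triggers game over for any flagged Trace.
; A looping one-second timer declares victory when the fruit count drops to the Spawner's threshold.
; Either outcome sets Spawner.GameOver, plays sound and optionally shows a Mahjong widget; defeat also desaturates post-processing via timeline.
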(event Custom|GameOver
  (bind _postprocess (Variables|Default|GetPostProcess))
  ;[1 1 1] GameOver
  (Components|Timeline|SetPlayRate (Variables|Default|GetTimeline_0) 1.0)
  (bind _newtrack_0 (Timeline|Timeline_0 PlayFromStart)
    (:Update
      (bind _output_get (Variables|Default|SetSaturation (Math|Float|Lerp 1.0 0.0 _newtrack_0)))
      (Variables|/Script/Engine.PostProcessComponent|SetSettings _postprocess (Utilities|Struct|MakePostProcessSettings (Math|Vector4|MakeVector4 (* (.X (Math|Vector4|BreakVector4 (Utilities|Struct|BreakPostProcessSettings (Variables|/Script/Engine.PostProcessComponent|GetSettings _postprocess)))) (.Y (Math|Vector4|BreakVector4 (Utilities|Struct|BreakPostProcessSettings (Variables|/Script/Engine.PostProcessComponent|GetSettings _postprocess)))) (.Z (Math|Vector4|BreakVector4 (Utilities|Struct|BreakPostProcessSettings (Variables|/Script/Engine.PostProcessComponent|GetSettings _postprocess)))) (.W (Math|Vector4|BreakVector4 (Utilities|Struct|BreakPostProcessSettings (Variables|/Script/Engine.PostProcessComponent|GetSettings _postprocess)))) _output_get) (* (.X (Math|Vector4|BreakVector4 (Utilities|Struct|BreakPostProcessSettings (Variables|/Script/Engine.PostProcessComponent|GetSettings _postprocess)))) (.Y (Math|Vector4|BreakVector4 (Utilities|Struct|BreakPostProcessSettings (Variables|/Script/Engine.PostProcessComponent|GetSettings _postprocess)))) (.Z (Math|Vector4|BreakVector4 (Utilities|Struct|BreakPostProcessSettings (Variables|/Script/Engine.PostProcessComponent|GetSettings _postprocess)))) (.W (Math|Vector4|BreakVector4 (Utilities|Struct|BreakPostProcessSettings (Variables|/Script/Engine.PostProcessComponent|GetSettings _postprocess)))) _output_get) (* (.X (Math|Vector4|BreakVector4 (Utilities|Struct|BreakPostProcessSettings (Variables|/Script/Engine.PostProcessComponent|GetSettings _postprocess)))) (.Y (Math|Vector4|BreakVector4 (Utilities|Struct|BreakPostProcessSettings (Variables|/Script/Engine.PostProcessComponent|GetSettings _postprocess)))) (.Z (Math|Vector4|BreakVector4 (Utilities|Struct|BreakPostProcessSettings (Variables|/Script/Engine.PostProcessComponent|GetSettings _postprocess)))) (.W (Math|Vector4|BreakVector4 (Utilities|Struct|BreakPostProcessSettings (Variables|/Script/Engine.PostProcessComponent|GetSettings _postprocess)))) _output_get) (* (.X (Math|Vector4|BreakVector4 (Utilities|Struct|BreakPostProcessSettings (Variables|/Script/Engine.PostProcessComponent|GetSettings _postprocess)))) (.Y (Math|Vector4|BreakVector4 (Utilities|Struct|BreakPostProcessSettings (Variables|/Script/Engine.PostProcessComponent|GetSettings _postprocess)))) (.Z (Math|Vector4|BreakVector4 (Utilities|Struct|BreakPostProcessSettings (Variables|/Script/Engine.PostProcessComponent|GetSettings _postprocess)))) (.W (Math|Vector4|BreakVector4 (Utilities|Struct|BreakPostProcessSettings (Variables|/Script/Engine.PostProcessComponent|GetSettings _postprocess)))) _output_get))))
      (Utilities|FlowControl|DoOnce false
        (:Completed
          (Audio|PlaySound2D "/Game/Square/Audio/失败.失败" 1.0 1.0 0.0 0 0)
          (Variables|/Game/Combine/BP/BP_Spawner.BP_Spawner_C|SetGameOver (Variables|Default|GetSpawner) true)
          (if (Variables|Default|GetUI)
            (bind _returnvalue (UserInterface|CreateWidget "/Game/Mahjong/BP/UI_Fail_Mahjong.UI_Fail_Mahjong_C"))
            (UserInterface|Viewport|AddtoViewport _returnvalue 0)))))))

(event Custom|Victory
  (bind _outactors (Actor|GetAllActorsOfClass "/Game/Combine/BP/BP_FruitMaster.BP_FruitMaster_C"))
  (if (<= (Utilities|Array|Length _outactors) (Variables|/Game/Combine/BP/BP_Spawner.BP_Spawner_C|Get胜利条件 (Variables|Default|GetSpawner)))
    (Utilities|FlowControl|DoOnce false
      (:Completed
        (Variables|Default|SetVictory? true)
        (Variables|/Game/Combine/BP/BP_Spawner.BP_Spawner_C|SetGameOver (Variables|Default|GetSpawner) true)
        (Audio|PlaySound2D "/Game/Square/Audio/UI_的胜利.UI_的胜利" 1.0 1.0 0.0 0 0)
        (if (Variables|Default|GetUI)
          (bind _returnvalue (UserInterface|CreateWidget "/Game/Mahjong/BP/UI_Victory_Mahjong.UI_Victory_Mahjong_C"))
          (UserInterface|Viewport|AddtoViewport _returnvalue 0))))))

(event EventBeginPlay
  (bind _returnvalue (Actor|GetActorOfClass "/Game/Combine/BP/BP_Spawner.BP_Spawner_C"))
  (Variables|Default|SetSpawner _returnvalue)
  (Utilities|Time|SetTimerbyEvent (delegate Custom|Victory) 1.0 true)
  (Utilities|FlowControl|Delay 2.0)
  (Variables|Default|SetDelay true))

(event Collision|EventActorBeginOverlap
  (params (OtherActor :type Actor%20Object%20Reference)))

(event EventTick
  (params (DeltaSeconds :type Float%20%28single-precision%29))
  (if (Variables|Default|GetDelay)
    (for _array_element (Collision|GetOverlappingActors (Variables|Default|GetBox) "/Game/Combine/BP/BP_FruitMaster.BP_FruitMaster_C" :!class /Script/Engine.PrimitiveComponent)
      (bind _asbp_fruit_master (Utilities|Casting|CastToBP_FruitMaster _array_element))
      (if (Variables|/Game/Combine/BP/BP_FruitMaster.BP_FruitMaster_C|GetTrace _asbp_fruit_master)
        (Utilities|FlowControl|DoOnce false
          (:Completed
            (CallFunction|GameOver)))))))

(fn ConstructionScript
  (Components|Box|SetBoxExtent (Variables|Default|GetBox) (Variables|Default|GetIn%20Box%20Extent) true))