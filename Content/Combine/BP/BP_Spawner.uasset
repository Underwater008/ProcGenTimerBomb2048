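; BP_Spawner is the dropper in a fruit-combining game, spawning BP_FruitMaster pieces and releasing them on a timed loop.
; Spawn nudges its position by a random positive X/Y offset, then attaches a non-colliding fruit with random or fixed level.
; ReleaseTimer enables physics and collision, detaches the fruit, then respawns and repeats after random delays until GameOver.
; Holding A or D slides it sideways by a fixed step per Tick.
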(event Custom|_ReleaseTimer
  (bind _bp_fruit (Variables|Default|GetBP%20Fruit))
  (bind _box (Variables|/Game/Combine/BP/BP_FruitMaster.BP_FruitMaster_C|GetBox _bp_fruit))
  ;[1 1 1] Control
  (if (not (Variables|Default|GetGameOver))
    (Utilities|IsValid _bp_fruit
      (:Is%20Valid
        (Physics|SetSimulatePhysics _box true)
        (Variables|/Game/Combine/BP/BP_FruitMaster.BP_FruitMaster_C|SetSimulate _bp_fruit true)
        (Collision|SetCollisionEnabled _box "QueryAndPhysics")
        (Transformation|DetachFromActor _bp_fruit "KeepWorld" "KeepWorld" "KeepWorld")
        (Audio|PlaySound2D "/Game/Square/Audio/下落.下落" 1.0 1.0 0.0 0 0)
        (Utilities|FlowControl|Delay (Math|Random|RandomFloatinRange 2.0 5.0))
        (CallFunction|Spawn)
        (Utilities|FlowControl|Delay (Math|Random|RandomFloatinRange 2.0 5.0))
        (CallFunction|ReleaseTimer)))))

(event EventBeginPlay
  (Input|EnableInput (Game|GetPlayerController 0))
  (CallFunction|Spawn)
  (Utilities|FlowControl|Delay 0.5)
  (CallFunction|ReleaseTimer))

(event Collision|EventActorBeginOverlap
  (params (OtherActor :type Actor%20Object%20Reference)))

(event EventTick
  (params (DeltaSeconds :type Float%20%28single-precision%29))
  (bind _returnvalue (Transformation|GetActorRightVector))
  (if (Variables|Default|GetMove)
    (Transformation|AddActorWorldOffset (select (Variables|Default|GetLeft/Right) (* _returnvalue -5.0) (* _returnvalue 5.0)))))

(event Input|KeyboardEvents|A
  (params (Key :type Key%20Structure :default "None"))
  ;[1 1 1] Control
  (:Pressed
    (if (not (Variables|Default|GetGameOver))
      (Variables|Default|SetMove true)
      (Variables|Default|SetLeft/Right true)
      (Audio|PlaySound2D "/Game/Square/Audio/上升_.上升_" 1.0 1.0 0.0 0 0)))
  (:Released
    (Variables|Default|SetMove false)))

(event Input|KeyboardEvents|D
  (params (Key :type Key%20Structure :default "None"))
  ;[1 1 1] Control
  (:Pressed
    (if (not (Variables|Default|GetGameOver))
      (Variables|Default|SetMove true)
      (Variables|Default|SetLeft/Right false)
      (Audio|PlaySound2D "/Game/Square/Audio/上升_.上升_" 1.0 1.0 0.0 0 0)))
  (:Released
    (Variables|Default|SetMove false)))

(event Input|KeyboardEvents|SpaceBar
  (params (Key :type Key%20Structure :default "None"))
  ;[1 1 1] Control
)

(fn ConstructionScript)

(fn Spawn
  (Transformation|SetActorLocation (+ (Transformation|GetActorLocation) (Math|Vector|MakeVector (Math|Random|RandomFloatinRange 3e+01 1.2e+02) (Math|Random|RandomFloatinRange 3e+01 1.2e+02) 0.0)) false false)
  (bind _returnvalue (Game|SpawnActorfromClass "/Game/Combine/BP/BP_FruitMaster.BP_FruitMaster_C" (Math|Transform|MakeTransform (Transformation|GetActorLocation) "0, 0, 0" "1.000000,1.000000,1.000000") "AlwaysSpawn" 0 (select (Variables|Default|Get随机模式) (.OutItem (Utilities|Array|Random (Utilities|Array|MakeArray "NewEnumerator0" "NewEnumerator1" "NewEnumerator2" "NewEnumerator3" "NewEnumerator4" "NewEnumerator5"))) (Variables|Default|Get固定生成)) (Variables|Default|Get游戏模式) false 1000 9999 0))
  (bind _output_get (Variables|Default|SetBP%20Fruit _returnvalue))
  (Variables|/Game/Combine/BP/BP_FruitMaster.BP_FruitMaster_C|SetTrace _output_get false)
  (Transformation|AttachActorToActor _output_get self "None" "KeepWorld" "KeepWorld" "KeepWorld" true)
  (Collision|SetCollisionEnabled (Variables|/Game/Combine/BP/BP_FruitMaster.BP_FruitMaster_C|GetBox _output_get) "NoCollision"))